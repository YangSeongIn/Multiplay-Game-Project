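; BP_Test_Tick is a test actor that continuously moves up and down between its starting height and 1000 units above it.
; BeginPlay stores both heights, and Tick eases the current Z toward the active target with FInterpTo, keeping X and Y unchanged.
; When the height comes within a small tolerance of either end, the target flips to the opposite one.
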(event `self.ReceiveBeginPlay`
  (bind (_returnvalue_x _returnvalue_y _returnvalue_z) (`KismetMathLibrary.BreakVector` (`self.K2_GetActorLocation`)))
  (bind _output_get (set `self.TargetPos` (+ _returnvalue_z 1000.0)))
  (set `self.CurTargetPos` _output_get)
  (set `self.InitPos` _returnvalue_z)
  (set `self.CurrentPos` _returnvalue_z))

(event `self.ReceiveTick`
  (params (DeltaSeconds :type "Float (single-precision)"))
  (bind (_returnvalue_x _returnvalue_y) (`KismetMathLibrary.BreakVector` (`self.K2_GetActorLocation`)))
  (bind _returnvalue (`KismetMathLibrary.FInterpTo` (`self.CurrentPos`) (`self.CurTargetPos`) DeltaSeconds 2.0))
  (if (`KismetMathLibrary.NearlyEqual_FloatFloat` (`self.CurrentPos`) (`self.TargetPos`) 3.0)
    (set `self.CurTargetPos` (`self.InitPos`))
    (elif (`KismetMathLibrary.NearlyEqual_FloatFloat` (`self.CurrentPos`) (`self.InitPos`) 3.0)
      (set `self.CurTargetPos` (`self.TargetPos`))))
  (`self.K2_SetActorLocation` (`KismetMathLibrary.MakeVector` _returnvalue_x _returnvalue_y _returnvalue))
  (set `self.CurrentPos` _returnvalue))

(fn `UserConstructionScript`)