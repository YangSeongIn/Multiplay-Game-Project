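; Lobby camera actor that glides between a lobby view and a character or item customization view.
; Each Tick checks two flags, with ActivateToCustomize taking priority over ActivateToLobby, and calls the matching move function.
; Both functions use TInterpTo to ease the actor transform toward a hardcoded location and rotation, without sweep.
; The flags are only read here, never set.
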(event `self.ReceiveTick`
  (params (DeltaSeconds :type "Float (single-precision)"))
  (if (`self.bActivateToCustomize`)
    (`self.SetLocationToCustomize` DeltaSeconds)
    (elif (`self.bActivateToLobby`)
      (`self.SetLocationToLobby` DeltaSeconds))))

(fn `SetLocationToCustomize`
  (params (DeltaTime :type "Float (double-precision)"))
  (`self.K2_SetActorTransform` (`KismetMathLibrary.TInterpTo` (`self.GetTransform`) (`KismetMathLibrary.MakeTransform` (62.0 270.0 190.0) (struct :`Pitch` -10.0 :`Yaw` -120.0)) DeltaTime 6.0)))

(fn `SetLocationToLobby`
  (params (DeltaTime :type "Float (double-precision)"))
  (`self.K2_SetActorTransform` (`KismetMathLibrary.TInterpTo` (`self.GetTransform`) (`KismetMathLibrary.MakeTransform` (0.0 350.0 110.0) (struct :`Pitch` 10.0 :`Yaw` -90.0)) DeltaTime 6.0)))

(fn `UserConstructionScript`)